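; Trader NPC that walks to the player's base gates, offers trading, and heads to the exit location when the trade ends.
; On BeginPlay it stocks its inventory and steers its AI by writing CrewManager-provided locations to the TargetLocation Blackboard key.
; Interaction starts a dialog, while trade start opens character, trader, buy and sell inventories through the game mode's UiManager.
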(event EventBeginPlay
  (bind _inventory (Variables|Default|GetInventory))
  (Utilities|FlowControl|Delay 0.2)
  (Class|InventoryComponent|AddItem _inventory (Utilities|Struct|MakeItemInstance "/Game/DataAssets/Items/Consumable/AppleItem.AppleItem" 2))
  (Class|InventoryComponent|AddItem _inventory (Utilities|Struct|MakeItemInstance "/Game/DataAssets/Items/AxeItem.AxeItem" 5))
  ;[1 1 1] Go to Player's gates
  (Utilities|FlowControl|Delay -1.0)
  (CallFunction|GotoLocation (Default|GetPlayerBaseEntranceLocation (.AsCrew%20Manager%20BP (Utilities|Casting|CastToCrewManagerBP (Variables|/Script/Survival.PlayerGameMode|GetcrewManager (.AsPlayer%20Game%20Mode (Utilities|Casting|CastToPlayerGameMode (Game|GetGameMode)))))))))

(fn ConstructionScript
  (Transformation|AttachComponentToComponent (Variables|Default|GetBackpack) (Variables|Character|GetMesh) "Backpack" "KeepRelative" "KeepRelative" "KeepRelative" true))

(fn OnTradeStart
  (params (Character :type AI%20Character%20Object%20Reference))
  (bind _returnvalue (Game|GetGameMode))
  (bind _asplayer_game_mode_bp (Utilities|Casting|CastToPlayerGameModeBP _returnvalue))
  (bind _uimanager (Variables|/Script/Survival.PlayerGameMode|GetuiManager _asplayer_game_mode_bp))
  (Class|UIManager|OpenInventory _uimanager (Variables|/Script/Survival.AICharacter|GetinventoryComp Character) (Utilities|Enum|LiteralenumEInventoryOpenType "Single"))
  (Class|UIManager|OpenInventory _uimanager (Variables|Default|GetInventory) (Utilities|Enum|LiteralenumEInventoryOpenType "Exchange"))
  (Class|UIManager|OpenInventory _uimanager (Variables|Default|GetPlayerSellInventory) (Utilities|Enum|LiteralenumEInventoryOpenType "TradePlayerSell"))
  (Class|UIManager|OpenInventory _uimanager (Variables|Default|GetPlayerBuyInventory) (Utilities|Enum|LiteralenumEInventoryOpenType "TradePlayerBuy")))

(fn OnTradeEnd
  (CallFunction|GoBack)
  (Development|PrintString "Trade ended"))

(fn GotoLocation
  (params (Location :type Vector))
  (AI|Components|Blackboard|SetValueasVector (AI|GetBlackboard 0) (Utilities|Name|MakeLiteralName "TargetLocation") Location))

(fn GoBack
  (Variables|Default|SetIsGoingBack true)
  (CallFunction|GotoLocation (Default|GetCharacterExitLocation (.AsCrew%20Manager%20BP (Utilities|Casting|CastToCrewManagerBP (Variables|/Script/Survival.PlayerGameMode|GetcrewManager (.AsPlayer%20Game%20Mode (Utilities|Casting|CastToPlayerGameMode (Game|GetGameMode)))))))))

(fn GetAnimType
  (return "Default"))

(fn GetCanbeInteracted
  (return true))

(fn InteractionTick
  (params (deltaSeconds :type Float%20%28single-precision%29%20%28by%20ref%29) (character :type AI%20Character%20Object%20Reference))
  (Class|DialogInvokerComponent|StartDialog (Variables|Default|GetDialogInvoker) character)
  (return true))