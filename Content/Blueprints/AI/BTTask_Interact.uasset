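; Behavior tree task that makes an AI character interact with the actor stored in the InteractableActor blackboard value.
; On execute, the controlled BPAICharacter turns to look at that actor.
; Each tick it passes the actor, cast to Interactable, to the character's ControlInteractableForTask, and finishes successfully once that returns true.
; The task itself has no failure path.
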(event EventReceiveExecute
  (params (OwnerActor :type Actor%20Object%20Reference))
  (Class|AICharacter|LookatActor (.AsBPAICharacter (Utilities|Casting|CastToBPAICharacter (Pawn|GetControlledPawn (.AsBPAIController (Utilities|Casting|CastToBPAIController OwnerActor))))) (AI|BehaviorTree|GetBlackboardValueasActor (Variables|Default|GetInteractableActor))))

(event EventTick
  (params (OwnerActor :type Actor%20Object%20Reference) (DeltaSeconds :type Float%20%28single-precision%29))
  (bind _isfinished (Default|ControlInteractableforTask (.AsBPAICharacter (Utilities|Casting|CastToBPAICharacter (Pawn|GetControlledPawn (.AsBPAIController (Utilities|Casting|CastToBPAIController OwnerActor))))) DeltaSeconds (.AsInteractable (Utilities|Casting|CastToInteractable (AI|BehaviorTree|GetBlackboardValueasActor (Variables|Default|GetInteractableActor))))))
  (if _isfinished
    (AI|BehaviorTree|FinishExecute true)))