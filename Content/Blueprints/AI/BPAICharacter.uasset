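; AI crew character Blueprint that registers with the game mode's CrewManager on spawn and unregisters when destroyed.
; Each tick it walks to a target location, or to a target actor within its interaction distance, turning to face it.
; At the target it feeds build and destruction speeds into the actor's InteractionTick, flagging itself as interacting.
; When that completes on a DestructibleBase, it collects the drop items into its inventory and destroys the actor.
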(event EventBeginPlay
  (Crew|AddtoCrew))

(event EventDestroyed
  (Crew|RemovefromCrew))

(event EventTick
  (params (DeltaSeconds :type Float%20%28single-precision%29))
  (bind _self self)
  (bind _targetactor (Variables|Default|GettargetActor))
  (bind _returnvalue (AI|GetAIController _self))
  (Class|AICharacter|SetIsInteracting (Class|KismetSystemLibrary|MakeLiteralBool false))
  (if (Utilities|IsValid _targetactor)
    (CallFunction|ControlInteractable _returnvalue (Variables|/Script/Survival.InteractableBase|GetinteractionDistance _targetactor) DeltaSeconds)
    (Class|AICharacter|LookatTargetActor)
    (else
      (AI|Navigation|MovetoLocation _returnvalue (Variables|Default|GettargetLocation) -1.0 true true false true 0))))

(fn ConstructionScript)

(fn AddtoCrew
  (Default|AddMember (Variables|/Script/Survival.PlayerGameMode|GetcrewManager (.AsPlayer%20Game%20Mode%20BP (Utilities|Casting|CastToPlayerGameModeBP (Game|GetGameMode)))) self))

(fn RemovefromCrew
  (Class|CrewManager|RemoveMember (Variables|/Script/Survival.PlayerGameMode|GetcrewManager (.AsPlayer%20Game%20Mode%20BP (Utilities|Casting|CastToPlayerGameModeBP (Game|GetGameMode)))) self))

(fn ControlInteractable
  (params (AIController :type AI%20Controller%20Object%20Reference) (AcceptanceRadius :type Float%20%28single-precision%29) (DeltaSeconds :type Float%20%28single-precision%29))
  (bind _targetactor (Variables|Default|GettargetActor))
  (bind _targetactor_2 (Variables|Default|GettargetActor))
  (bind (_asdestructible_base _bsuccess) (Utilities|Casting|CastToDestructibleBase _targetactor))
  (bind _returnvalue (AI|Navigation|MovetoActor AIController _targetactor_2 AcceptanceRadius true true true 0))
  (if (Utilities|Enum|Equal(Enum) _returnvalue "AlreadyAtGoal")
    (bind _returnvalue_2 (Class|InteractableBase|InteractionTick _targetactor_2 DeltaSeconds (Variables|Default|GetdestructionSpeed) (Variables|Default|GetbuildSpeed)))
    (if _returnvalue_2
      (if _bsuccess
        (Class|InventoryComponent|AddItemsfromAsset (Variables|Default|GetinventoryComponent) (Variables|/Script/Survival.DestructibleBase|GetafterDestroyItems _asdestructible_base))
        (Actor|DestroyActor _asdestructible_base))
      (else
        (Class|AICharacter|SetIsInteracting (Class|KismetSystemLibrary|MakeLiteralBool true))))))