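; Base Blueprint for AI crew characters, which register with the game mode's CrewManager on BeginPlay and leave it when destroyed.
; Each tick clears the interacting flag and adds a bleeding status when happiness is low.
; ControlInteractableForTask runs a target's normal or destruction interaction, setting that flag while it returns false.
; The character is also interactable itself, starting a conversation through the ConversationManager.
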(event EventBeginPlay
  (Crew|AddtoCrew))

(event EventDestroyed
  (Crew|RemovefromCrew))

(event EventTick
  (params (DeltaSeconds :type Float%20%28single-precision%29))
  (Class|AICharacter|SetIsInteracting (Class|KismetSystemLibrary|MakeLiteralBool false))
  ;[1 1 1] Add bleeding status when happyness is low
  (if (< (Class|Statistic|GetAmountNormalized (Class|NPCNeeds|GetNeedbyType (Class|AICharacter|GetNeeds) "Happyness")) 0.2)
    (Class|NPCStatuses|AddStatus (Class|AICharacter|GetStatuses) "/Game/DataAssets/Statuses/BleedingStatus.BleedingStatus")))

(fn ConstructionScript)

(fn AddtoCrew
  (Default|AddMember (Variables|/Script/Survival.PlayerGameMode|GetcrewManager (.AsPlayer%20Game%20Mode%20BP (Utilities|Casting|CastToPlayerGameModeBP (Game|GetGameMode)))) self))

(fn RemovefromCrew
  (Class|CrewManager|RemoveMember (Variables|/Script/Survival.PlayerGameMode|GetcrewManager (.AsPlayer%20Game%20Mode%20BP (Utilities|Casting|CastToPlayerGameModeBP (Game|GetGameMode)))) self))

(fn ControlInteractableforTask
  (params (DeltaSeconds :type Float%20%28single-precision%29) (TargetInteractable :type Interactable%20Interface))
  (bind _self self)
  (switch Utilities|FlowControl|Switch|SwitchonEInteractionType (Class|AICharacter|GetInteractionType _self)
    (:Default
      (bind _returnvalue (Class|Interactable|InteractionTick TargetInteractable DeltaSeconds _self))
      (if _returnvalue
        _
        (else
          (Class|AICharacter|SetIsInteracting (Class|KismetSystemLibrary|MakeLiteralBool true) :!label _label)
          (return false))))
    (:Destruction
      (bind _asinteractable_base (Utilities|Casting|CastToInteractableBase TargetInteractable)
        (:then
          (bind _returnvalue_2 (Class|InteractableBase|DestructionInteraction _asinteractable_base DeltaSeconds _self))
          (if _returnvalue_2
            _
            (else
              (goto _label))))
        (:CastFailed
          (Development|PrintString "Interaction type is Destruction, but target actor isn't InteractableBase")
          (return false)))))
  (return true))

(fn InteractionTick
  (params (deltaSeconds :type Float%20%28single-precision%29%20%28by%20ref%29) (character :type AI%20Character%20Object%20Reference))
  (Class|ConversationManager|StartConversation (Variables|/Script/Survival.PlayerGameMode|GetconversationManager (.AsPlayer%20Game%20Mode (Utilities|Casting|CastToPlayerGameMode (Game|GetGameMode)))) character self)
  (return true))