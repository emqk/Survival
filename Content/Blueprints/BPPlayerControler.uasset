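; Player camera and input actor for a game where the player selects AI characters, directs their interactions and places buildings.
; Each tick it pans, zooms within height limits, rotates on middle-mouse with clamped pitch, and feeds the cursor hit to the BuildingManager.
; Clicks confirm or cancel building, otherwise select an NPC or open the UiManager interaction widget, whose answer goes to that NPC.
; Hovered Interactables get outlined through custom depth stencil.
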(event EventBeginPlay
  (bind _returnvalue (Transformation|GetActorRotation))
  (bind (_roll _pitch _yaw) (Math|Rotator|BreakRotator _returnvalue))
  (CallFunction|ClampRotation (Math|Rotator|MakeRotator _roll (Variables|Rotation|GetStartAngle) _yaw)))

(event EventTick
  (params (DeltaSeconds :type Float%20%28single-precision%29))
  (CallFunction|Movement DeltaSeconds)
  (CallFunction|Rotation DeltaSeconds)
  (Building|TickBuilding)
  (CallFunction|TickOutline))

(event Input|MouseEvents|RightMouseButton
  (params (Key :type Key%20Structure :default "None"))
  (bind _hitresult (CallFunction|GetCursorHitResult))
  (bind (_bblockinghit _binitialoverlap _time _distance _location _impactpoint _normal _impactnormal _physmat _hitactor) (Collision|BreakHitResult _hitresult))
  (:Pressed
    (if (Class|BuildingManager|IsBuilding (Variables|/Script/Survival.PlayerGameMode|GetbuildingManager (.AsPlayer%20Game%20Mode%20BP (Utilities|Casting|CastToPlayerGameModeBP (Game|GetGameMode)))))
      (Building|CancelBuilding)
      (elif (CallFunction|IsNPCSelected)
        (bind _asinteractable (Utilities|Casting|CastToInteractable _hitactor)
          (:then
            (bind _result (CallFunction|IsThisSelectedNPCActor _asinteractable))
            (if (not _result)
              (Interaction|SetInteractionWidgetActor _hitactor)))
          (:CastFailed
            (Interaction|SetInteractionWidgetLocation _location)))))))

(event Input|MouseEvents|LeftMouseButton
  (params (Key :type Key%20Structure :default "None"))
  (:Pressed
    (if (Class|BuildingManager|IsBuilding (Variables|/Script/Survival.PlayerGameMode|GetbuildingManager (.AsPlayer%20Game%20Mode%20BP (Utilities|Casting|CastToPlayerGameModeBP (Game|GetGameMode)))))
      (Building|EndBuilding)
      (else
        (NPC|ControlCharacters)))))

(event Input|KeyboardEvents|X
  (params (Key :type Key%20Structure :default "None"))
  ;[1 1 1] Scavenge
  (:Pressed
    (Class|UIManager|ToggleScavengePanel (Variables|/Script/Survival.PlayerGameMode|GetuiManager (.AsPlayer%20Game%20Mode%20BP (Utilities|Casting|CastToPlayerGameModeBP (Game|GetGameMode)))))))

(event Input|KeyboardEvents|CapsLock
  (params (Key :type Key%20Structure :default "None"))
  ;[1 1 1] Settings
  (:Pressed
    (Class|UIManager|ToggleSettingsPanel (Variables|/Script/Survival.PlayerGameMode|GetuiManager (.AsPlayer%20Game%20Mode%20BP (Utilities|Casting|CastToPlayerGameModeBP (Game|GetGameMode)))))))

(event Input|KeyboardEvents|Q
  (params (Key :type Key%20Structure :default "None"))
  ;[1 1 1] Testing architecture building
  (:Pressed
    (Class|BuildingManager|ChangeRotationY (Variables|/Script/Survival.PlayerGameMode|GetbuildingManager (.AsPlayer%20Game%20Mode%20BP (Utilities|Casting|CastToPlayerGameModeBP (Game|GetGameMode)))) (Math|Float|MakeLiteralFloat -9e+01))))

(event Input|KeyboardEvents|E
  (params (Key :type Key%20Structure :default "None"))
  ;[1 1 1] Testing architecture building
  (:Pressed
    (Class|BuildingManager|ChangeRotationY (Variables|/Script/Survival.PlayerGameMode|GetbuildingManager (.AsPlayer%20Game%20Mode%20BP (Utilities|Casting|CastToPlayerGameModeBP (Game|GetGameMode)))) (Math|Float|MakeLiteralFloat 9e+01))))

(fn ConstructionScript)

(fn Movement
  (params (DeltaSeconds :type Float%20%28single-precision%29))
  (bind _returnvalue (Transformation|GetActorRotation))
  (bind _returnvalue_2 (Transformation|GetActorLocation))
  (bind _returnvalue_3 (Class|Actor|GetInputAxisKeyValue))
  (bind _mousewheelspeed (Variables|Movement|GetMouseWheelSpeed))
  (bind (_roll _pitch _yaw) (Math|Rotator|BreakRotator _returnvalue))
  (bind _returnvalue_4 (* -1 _returnvalue_3))
  (bind _returnvalue_5 (* _returnvalue_4 _mousewheelspeed))
  (bind _returnvalue_6 (Math|Vector|MakeVector 0.0 0.0 _returnvalue_5))
  (bind _returnvalue_7 (+ _returnvalue_6 _returnvalue_2))
  (bind (_x _y _z) (Math|Vector|BreakVector _returnvalue_7))
  ;[1 1 1] Movement
  (LocalVariables|SetMoveVector (* (Transformation|GetActorRightVector) (Input|AxisValues|GetHorizontal)))
  (bind _output_get (LocalVariables|SetMoveVector (+ (LocalVariables|GetMoveVector) (* (Math|Vector|RotateVector (Math|Vector|MakeVector 1.0 0.0 0.0) (Math|Rotator|MakeRotator _roll 0.0 _yaw)) (Input|AxisValues|GetVertical)))))
  (Transformation|AddActorWorldOffset (* (Math|Vector|Normalize _output_get) (* (Variables|Movement|GetMovementSpeed) DeltaSeconds)))
  ;[1 1 1] Zoom
  (Transformation|SetActorLocation (Math|Vector|MakeVector _x _y (Math|Float|Clamp(Float) _z (Variables|Movement|GetMinHeight) (Variables|Movement|GetMaxHeight))) false false))

(fn Rotation
  (params (DeltaSeconds :type Float%20%28single-precision%29))
  (bind _returnvalue (Transformation|GetActorRotation))
  (bind (_roll _pitch _yaw) (Math|Rotator|BreakRotator _returnvalue))
  (if (Game|Player|IsInputKeyDown (Game|GetPlayerController 0) "MiddleMouseButton")
    (CallFunction|ClampRotation (Math|Rotator|MakeRotator _roll (+ (* (* (Class|Actor|GetInputAxisKeyValue) DeltaSeconds) (Variables|Rotation|GetRotateSpeed)) _pitch) (+ _yaw (* (* (Class|Actor|GetInputAxisKeyValue) DeltaSeconds) (Variables|Rotation|GetRotateSpeed)))))))

(fn ControlCharacters
  (bind _asbpaicharacter (Utilities|Casting|CastToBPAICharacter (.HitActor (Collision|BreakHitResult (CallFunction|GetCursorHitResult)))))
  (NPC|SelectNPC _asbpaicharacter))

(fn ClampRotation
  (params (Rotation :type Rotator))
  (bind (_roll _pitch _yaw) (Math|Rotator|BreakRotator Rotation))
  (Transformation|SetActorRotation (Math|Rotator|MakeRotator _roll (Math|Float|Clamp(Float) _pitch (Variables|Rotation|GetMinLookAngle) (Variables|Rotation|GetMaxLookAngle)) _yaw)))

(fn SelectNPC
  (params (NPC :type AI%20Character%20Object%20Reference))
  (Variables|NPC|SetSelectedAICharacter NPC)
  (NPC|UpdateSelectedNPC)
  (Audio|PlaySoundatLocation (Variables|Interaction|GetSelectCharacterSound) (Transformation|GetActorLocation) "0, 0, 0" 1.0 1.0 0.0 0 0 0))

(fn LookatNPC
  (params (NPC :type AI%20Character%20Object%20Reference))
  (bind _returnvalue (Transformation|GetActorLocation NPC))
  (bind (_x _y) (Math|Vector|BreakVector _returnvalue))
  (Transformation|SetActorLocation (Math|Vector|MakeVector (- _x (Variables|Movement|GetLookAtXOffset)) _y (Variables|Movement|GetLookAtHeight)) false false)
  (CallFunction|ClampRotation (Math|Rotator|FindLookatRotation (Transformation|GetActorLocation) _returnvalue)))

(fn GetCursorHitResult
  (return (.HitResult (Class|PlayerController|GetHitResultUnderCursorforObjects (Game|GetPlayerController 0) (Utilities|Array|MakeArray "ObjectTypeQuery1" "ObjectTypeQuery3") true))))

(fn SetInteractionWidgetLocation
  (params (Location :type Vector))
  (Class|UIManager|SetInteractionWidgetLocation (Variables|/Script/Survival.PlayerGameMode|GetuiManager (.AsPlayer%20Game%20Mode%20BP (Utilities|Casting|CastToPlayerGameModeBP (Game|GetGameMode)))) Location)
  (Variables|Interaction|SetIsWaitingForInteractionAnswer true))

(fn CatchInteractionAnswer
  (params (Location :type Vector) (Actor :type Actor%20Object%20Reference))
  (Class|AICharacter|SetInteraction (Variables|NPC|GetSelectedAICharacter) Location Actor)
  (Variables|Interaction|SetIsWaitingForInteractionAnswer false))

(fn SetInteractionWidgetActor
  (params (Actor :type Actor%20Object%20Reference))
  (Class|UIManager|SetInteractionWorldActor (Variables|/Script/Survival.PlayerGameMode|GetuiManager (.AsPlayer%20Game%20Mode%20BP (Utilities|Casting|CastToPlayerGameModeBP (Game|GetGameMode)))) Actor)
  (Variables|Interaction|SetIsWaitingForInteractionAnswer true))

(fn IsNPCSelected
  (return (Utilities|IsValid (Variables|NPC|GetSelectedAICharacter))))

(fn UpdateSelectedNPC
  (bind _selectedaicharacter (Variables|NPC|GetSelectedAICharacter))
  (Utilities|IsValid _selectedaicharacter
    (:Is%20Valid
      (Class|UIManager|RefreshNPCInfo (Variables|/Script/Survival.PlayerGameMode|GetuiManager (.AsPlayer%20Game%20Mode (Utilities|Casting|CastToPlayerGameMode (Game|GetGameMode)))) _selectedaicharacter))))

(fn IsThisSelectedNPCActor
  (params (Object :type Interactable%20Interface))
  (return (== (.AsActor (Utilities|Casting|CastToActor (.AsInteractable (Utilities|Casting|CastToInteractable (Variables|NPC|GetSelectedAICharacter))))) (.AsActor (Utilities|Casting|CastToActor Object)))))

(fn BeginBuilding
  (params (type :type Integer))
  (Class|BuildingManager|BeginBuilding (Variables|/Script/Survival.PlayerGameMode|GetbuildingManager (.AsPlayer%20Game%20Mode%20BP (Utilities|Casting|CastToPlayerGameModeBP (Game|GetGameMode))))))

(fn TickBuilding
  (Class|BuildingManager|TickBuilding (Variables|/Script/Survival.PlayerGameMode|GetbuildingManager (.AsPlayer%20Game%20Mode%20BP (Utilities|Casting|CastToPlayerGameModeBP (Game|GetGameMode)))) (.Location (Collision|BreakHitResult (CallFunction|GetCursorHitResult)))))

(fn EndBuilding
  (Class|BuildingManager|EndBuilding (Variables|/Script/Survival.PlayerGameMode|GetbuildingManager (.AsPlayer%20Game%20Mode%20BP (Utilities|Casting|CastToPlayerGameModeBP (Game|GetGameMode))))))

(fn CancelBuilding
  (Class|BuildingManager|CancelBuilding (Variables|/Script/Survival.PlayerGameMode|GetbuildingManager (.AsPlayer%20Game%20Mode%20BP (Utilities|Casting|CastToPlayerGameModeBP (Game|GetGameMode))))))

(fn TickOutline
  (bind _hitresult (CallFunction|GetCursorHitResult))
  (bind _hitactor (Collision|BreakHitResult _hitresult))
  (bind _returnvalue (Actor|GetComponentbyClass _hitactor "/Script/Engine.MeshComponent"))
  (Utilities|IsValid (Variables|Default|GetCurrentlyOutlinedMeshComp)
    (:Is%20Valid
      (Rendering|SetRenderCustomDepth (Variables|Default|GetCurrentlyOutlinedMeshComp) false)
      (Rendering|SetCustomDepthStencilValue (Variables|Default|GetCurrentlyOutlinedMeshComp) 0))
    (:Is%20Not%20Valid
      _))
  (Utilities|IsValid _hitactor
    (:Is%20Valid
      (Utilities|IsValid _returnvalue
        (:Is%20Valid
          (if (Utilities|DoesObjectImplementInterface _hitactor "/Script/Survival.Interactable")
            (Variables|Default|SetCurrentlyOutlinedMeshComp _returnvalue)
            (Rendering|SetRenderCustomDepth _returnvalue true)
            (Rendering|SetCustomDepthStencilValue _returnvalue 2)))))))