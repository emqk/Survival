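; Merchant is an interactable trader with its own inventory, which it stocks with apples and axes shortly after BeginPlay.
; InteractionTick uses the game mode's UiManager to open the character's inventory, the merchant's stock in Exchange mode, and separate player sell and buy inventories.
; Both the sell and buy inventories open with the TradePlayerSell type, and the interaction always returns true.
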(event EventBeginPlay
  (bind _inventory (Variables|Default|GetInventory))
  (Utilities|FlowControl|Delay 0.2)
  (Class|InventoryComponent|AddItem _inventory (Utilities|Struct|MakeItemInstance "/Game/DataAssets/Items/AppleItem.AppleItem" 2))
  (Class|InventoryComponent|AddItem _inventory (Utilities|Struct|MakeItemInstance "/Game/DataAssets/Items/AxeItem.AxeItem" 5)))

(event Collision|EventActorBeginOverlap
  (params (OtherActor :type Actor%20Object%20Reference)))

(event EventTick
  (params (DeltaSeconds :type Float%20%28single-precision%29)))

(fn ConstructionScript)

(fn InteractionTick
  (params (deltaSeconds :type Float%20%28single-precision%29%20%28by%20ref%29) (character :type AI%20Character%20Object%20Reference))
  (bind _returnvalue (Game|GetGameMode))
  (bind _asplayer_game_mode_bp (Utilities|Casting|CastToPlayerGameModeBP _returnvalue))
  (bind _uimanager (Variables|/Script/Survival.PlayerGameMode|GetuiManager _asplayer_game_mode_bp))
  (Class|UIManager|OpenInventory _uimanager (Variables|/Script/Survival.AICharacter|GetinventoryComp character) (Utilities|Enum|LiteralenumEInventoryOpenType "Single"))
  (Class|UIManager|OpenInventory _uimanager (Variables|Default|GetInventory) (Utilities|Enum|LiteralenumEInventoryOpenType "Exchange"))
  (Class|UIManager|OpenInventory _uimanager (Variables|Default|GetPlayerSellInventory) (Utilities|Enum|LiteralenumEInventoryOpenType "TradePlayerSell"))
  (Class|UIManager|OpenInventory _uimanager (Variables|Default|GetPlayerBuyInventory) (Utilities|Enum|LiteralenumEInventoryOpenType "TradePlayerSell"))
  (return true))