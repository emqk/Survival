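; BuildablePrototypeBP is the placeholder for an unbuilt furniture piece, holding collected materials and turning them into the finished actor.
; Setup applies visuals for the target class and fills a BuildingPrototypeWidget comparing build requirements against the inventory component.
; Once the inventory meets the requirements, character interaction ticks accumulate work at that character's build speed.
; At the work threshold, Build spawns the target class at the prototype's transform and plays a finish sound.
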(event EventRefreshText
  (Default|SetupTexts (.AsBuilding%20Prototype%20Widget (Utilities|Casting|CastToBuildingPrototypeWidget (UserInterface|GetUserWidgetObject (Variables|Default|GetmyWidget)))) (Variables|Default|GetbuildRequirements) (Variables|Default|GetinventoryComp)))

(fn ConstructionScript)

(fn Setup
  (params (ToBuildClass :type Buildable%20Base%20Class%20Reference))
  (Class|BuildablePrototype|SetupVisuals ToBuildClass)
  (Class|BuildablePrototype|RefreshText))

(fn Build
  (Game|SpawnActorfromClass (Variables|Default|GettoBuild) (Transformation|GetActorTransform) "Undefined" 0 0)
  (Audio|PlaySoundatLocation (Variables|Default|GetFinishBuildSound) (Transformation|GetActorLocation) "0, 0, 0" 1.0 1.0 0.0 0 0 0))

(fn InteractionTick
  (params (deltaSeconds :type Float%20%28single-precision%29%20%28by%20ref%29) (character :type AI%20Character%20Object%20Reference))
  (if (CallFunction|HaveRequiredItems)
    (bind _newparam (CallFunction|ConstructTick deltaSeconds 0.0 (Class|AICharacter|GetBuildSpeed character)))
    (return _newparam)))

(fn ConstructTick
  (params (DeltaSeconds :type Float%20%28single-precision%29) (DestructionSpeed :type Float%20%28single-precision%29) (BuildSpeed :type Float%20%28single-precision%29))
  (bind _output_get (Variables|Default|SetCurrentWorkAmount (+ (Variables|Default|GetCurrentWorkAmount) (* BuildSpeed DeltaSeconds))))
  (if (>= _output_get (Variables|Default|GetworkAmountToBuild))
    (CallFunction|Build)
    (return (>= _output_get (Variables|Default|GetworkAmountToBuild)))))

(fn HaveRequiredItems
  (return (Class|InventoryComponent|HaveAmountOfItems (Variables|Default|GetinventoryComp) (Variables|Default|GetbuildRequirements))))