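; BuildablePrototypeBP is a placeholder for a buildable that players construct through timed interaction.
; Setup applies the prototype mesh and material, stores the target class and fills a widget with build requirements.
; InteractionTick adds work through ConstructTick only while the inventory component holds the required items.
; Once enough work accumulates, Build spawns the target class at the same transform, destroys the prototype and plays a finish sound.
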(event EventBeginPlay)

(event Collision|EventActorBeginOverlap
  (params (OtherActor :type Actor%20Object%20Reference)))

(event EventTick
  (params (DeltaSeconds :type Float%20%28single-precision%29)))

(fn ConstructionScript)

(fn Setup
  (params (StaticMesh :type Static%20Mesh%20Object%20Reference) (ToBuildClass :type Buildable%20Base%20BP%20Class%20Reference))
  (Class|BuildablePrototype|SetupVisuals StaticMesh "/Game/Materials/BuildPrototypeMat.BuildPrototypeMat" ToBuildClass)
  (Default|SetupTexts (.AsBuilding%20Prototype%20Widget (Utilities|Casting|CastToBuildingPrototypeWidget (UserInterface|GetUserWidgetObject (Variables|Default|GetmyWidget)))) (Variables|Default|GetbuildRequirements)))

(fn Build
  (Game|SpawnActorfromClass (Variables|Default|GettoBuild) (Transformation|GetActorTransform) "Undefined" 0 0)
  (Actor|DestroyActor)
  (Audio|PlaySoundatLocation (Variables|Default|GetFinishBuildSound) (Transformation|GetActorLocation) "0, 0, 0" 1.0 1.0 0.0 0 0 0))

(fn InteractionTick
  (params (deltaSeconds :type Float%20%28single-precision%29%20%28by%20ref%29) (destructionSpeed :type Float%20%28single-precision%29%20%28by%20ref%29) (buildSpeed :type Float%20%28single-precision%29%20%28by%20ref%29))
  (if (CallFunction|HaveRequiredItems)
    (bind _newparam (CallFunction|ConstructTick deltaSeconds 0.0 buildSpeed))
    (return _newparam)))

(fn ConstructTick
  (params (DeltaSeconds :type Float%20%28single-precision%29) (DestructionSpeed :type Float%20%28single-precision%29) (BuildSpeed :type Float%20%28single-precision%29))
  (bind _output_get (Variables|Default|SetCurrentWorkAmount (+ (Variables|Default|GetCurrentWorkAmount) (* BuildSpeed DeltaSeconds))))
  (if (>= _output_get (Variables|Default|GetworkAmountToBuild))
    (CallFunction|Build)
    (return (>= _output_get (Variables|Default|GetworkAmountToBuild)))))

(fn HaveRequiredItems
  (return (Class|InventoryComponent|HaveAmountOfItems (Variables|Default|GetinventoryComp) (Variables|Default|GetbuildRequirements))))