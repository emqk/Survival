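; Crew manager Blueprint that tracks the player's crew members and controls the visiting trader.
; On BeginPlay it caches the exit and base entrance actors, then after a one-frame delay spawns Mark and Jason at random points with a default behavior tree.
; Adding or removing members refreshes the crew UI, and losing the last one shows the lost-game screen.
; It also spawns a single trader at the exit and can send it back.
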(event EventAddMember
  (params (member :type AI%20Character%20Object%20Reference))
  (Utilities|Array|Add (Variables|Default|Getmembers) member)
  (CallFunction|RefreshCrewWidget)
  (Development|PrintString "MemberAdded!" true true "(R=0.000000,G=0.572917,B=0.016377,A=1.000000)"))

(event EventRemoveMember
  (params (member :type AI%20Character%20Object%20Reference))
  (bind _returnvalue (Utilities|Array|RemoveItem (Variables|Default|Getmembers) member))
  (if _returnvalue
    (CallFunction|RefreshCrewWidget)
    (Development|PrintString "Member removed!" true true "(R=0.004252,G=1.000000,B=0.000000,A=1.000000)")
    (if (<= (Class|CrewManager|GetMembersCount) 0)
      (Default|ShowLostGame (.AsUIManager%20BP (Utilities|Casting|CastToUIManagerBP (Class|PlayerGameMode|GetUIManager (.AsPlayer%20Game%20Mode (Utilities|Casting|CastToPlayerGameMode (Game|GetGameMode)))))))
      (Audio|PlaySoundatLocation "/Game/Audio/Soundly/LostGame.LostGame" "0, 0, 0" "0, 0, 0" 1.0 1.0 0.0 0 0 0))
    (else
      (Development|PrintString "Member can't be removed!" true true "(R=1.000000,G=0.005617,B=0.000000,A=1.000000)"))))

(event EventBeginPlay
  (bind _returnvalue (Actor|GetActorOfClass "/Game/Blueprints/Crew/CharacterExitBP.CharacterExitBP_C"))
  (Variables|Default|SetCharacterExitPoint _returnvalue)
  (bind _returnvalue_2 (Actor|GetActorOfClass "/Game/Blueprints/Crew/PlayerBaseEntranceBP.PlayerBaseEntranceBP_C"))
  (Variables|Default|SetPlayerBaseEntrance _returnvalue_2)
  (Utilities|FlowControl|Delay -1.0) ; Wait one frame to setup CrewManager
  (CallFunction|SpawnNPCs "/Game/Blueprints/AI/CharacterVariations/MarkCharacter.MarkCharacter_C")
  (CallFunction|SpawnNPCs "/Game/Blueprints/AI/CharacterVariations/JasonCharacter.JasonCharacter_C"))

(fn ConstructionScript)

(fn RefreshCrewWidget
  (Class|UIManager|RefreshCrew (Variables|/Script/Survival.PlayerGameMode|GetuiManager (.AsPlayer%20Game%20Mode%20BP (Utilities|Casting|CastToPlayerGameModeBP (Game|GetGameMode)))) (Variables|Default|Getmembers)))

(fn SpawnNPCs
  (params (ToSpawn :type BPAI%20Character%20Base%20Class%20Reference))
  (AI|SpawnAIFromClass ToSpawn (Variables|Default|GetDefaultBehaviorTree) (Math|Vector|MakeVector (Math|Random|RandomFloatinRangefromStream -1.8e+03 -1.5e+03 (Math|Random|MakeRandomStream (Math|Random|RandomInteger 9999999))) (Math|Random|RandomFloatinRangefromStream -2e+02 2e+02 (Math|Random|MakeRandomStream (Math|Random|RandomInteger 9999999))) 2e+02) "0, 0, 0" true 0)
  (CallFunction|RefreshCrewWidget))

(fn SpawnTrader
  (if (CallFunction|IsTraderSpawned)
    (Development|PrintString "Can't spawn trader - Already spawned!" true true "(R=1.000000,G=0.000000,B=0.011574,A=1.000000)")
    (else
      (bind _returnvalue (AI|SpawnAIFromClass "/Game/Blueprints/AI/Trader/TraderBP.TraderBP_C" "/Game/Blueprints/AI/Trader/TraderBT.TraderBT" (CallFunction|GetCharacterExitLocation) "0, 0, 0" true 0))
      (Variables|Default|SetCurrentTrader (.AsTrader%20BP (Utilities|Casting|CastToTraderBP _returnvalue))))))

(fn GetCharacterExitLocation
  (return (Transformation|GetActorLocation (Variables|Default|GetCharacterExitPoint))))

(fn GetPlayerBaseEntranceLocation
  (return (Transformation|GetActorLocation (Variables|Default|GetPlayerBaseEntrance))))

(fn IsTraderSpawned
  (return (Utilities|IsValid (Variables|Default|GetCurrentTrader))))

(fn TraderGoBack
  (bind _currenttrader (Variables|Default|GetCurrentTrader))
  (Utilities|IsValid _currenttrader
    (:Is%20Valid
      (Default|GoBack _currenttrader))
    (:Is%20Not%20Valid
      (Development|PrintString "Trader can't go back - CurrentTrader is null!" true true "(R=1.000000,G=0.005650,B=0.000000,A=1.000000)"))))