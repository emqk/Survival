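; Game mode Blueprint that bootstraps the game's core manager actors when play begins.
; On BeginPlay it spawns the UI, crew, conversation, building and scavenge managers in sequence at the world origin.
; Each spawned manager is stored in a variable on the game mode, which holds the references to these systems.
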(event EventBeginPlay
  (bind _returnvalue (Math|Transform|MakeTransform "0, 0, 0"))
  (bind _returnvalue_2 (Game|SpawnActorfromClass 0 "/Game/Blueprints/UI/UIManagerBP.UIManagerBP_C" _returnvalue "Undefined" 0 0))
  (Variables|Default|SetuiManager _returnvalue_2)
  (bind _returnvalue_3 (Game|SpawnActorfromClass 0 "/Game/Blueprints/Crew/CrewManagerBP.CrewManagerBP_C" _returnvalue "Undefined" 0 0))
  (Variables|Default|SetcrewManager _returnvalue_3)
  (bind _returnvalue_4 (Game|SpawnActorfromClass 0 "/Script/Survival.ConversationManager" _returnvalue "Undefined" 0 0))
  (Variables|Default|SetconversationManager _returnvalue_4)
  (bind _returnvalue_5 (Game|SpawnActorfromClass 0 "/Game/Blueprints/Building/BuildingManagerBP.BuildingManagerBP_C" _returnvalue "Undefined" 0 0))
  (Variables|Default|SetbuildingManager _returnvalue_5)
  (bind _returnvalue_6 (Game|SpawnActorfromClass 0 "/Script/Survival.ScavengeManager" _returnvalue "Undefined" 0 0))
  (Variables|Default|SetscavengeManager _returnvalue_6))

(fn ConstructionScript)